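; BP_BaseLamp is a lamp actor with a switchable light, named as a base for lamps.
; SetLightEnabled stores the Enabled state and applies it to LightSource visibility, propagating to child components.
; ToggleLight inverts that state through the same event.
; The construction script applies Enabled when the actor is constructed, but BeginPlay always switches the light off.
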(event `self.ReceiveBeginPlay`
  ;[0.05 0.05 0.05 0.5] Begin Play
  (`self.Set Light Enabled` false))

(event `Set Light Enabled`
  (params (Enabled :type Boolean))
  ;[0.05 0.05 0.05 0.5] Set Light Enabled
  (bind _output_get (set `self.Enabled` Enabled))
  (`SceneComponent.SetVisibility` (`self.Light Source`) _output_get true))

(fn `Toggle Light`
  (`self.Set Light Enabled` (not (`self.Enabled`))))

(fn `UserConstructionScript`
  (`SceneComponent.SetVisibility` (`self.Light Source`) (`self.Enabled`) true))