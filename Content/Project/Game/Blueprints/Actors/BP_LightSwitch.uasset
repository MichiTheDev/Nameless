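; BP_LightSwitch is an interactable switch actor that toggles a linked lamp in the level.
; When its InteractableComponent fires OnInteract, it casts the Lamp reference to BP_Lamp and calls SwitchLight on it.
; On BeginPlay it prints a warning naming itself if no Lamp actor has been set.
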(event `self.ReceiveBeginPlay`
  (`/Engine/EditorBlueprintResources/StandardMacros.IsValid` (`self.Lamp`)
    (:`Is Not Valid`
      (`KismetSystemLibrary.PrintString` (`KismetStringLibrary.Concat_StrStr` (`KismetSystemLibrary.GetDisplayName` self) " has not set an actor as lamp")))))

(event `self.InteractableComponent.OnInteract`
  (params (Player :type "PlayerController Object Reference"))
  (`|ExecutionSequence`
    (:`then_1`
      (bind _asbp_lamp (cast `/Game/Project/Game/Blueprints/Actors/BP_Lamp` (`self.Lamp`)))
      (`/Game/Project/Game/Blueprints/Actors/BP_Lamp.Switch Light` _asbp_lamp))))

(fn `UserConstructionScript`)