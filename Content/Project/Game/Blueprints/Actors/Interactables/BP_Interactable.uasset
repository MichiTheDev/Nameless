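; BP_Interactable is an interactable actor that can toggle an outline on its mesh and respond to an interaction.
; ShowOutline and HideOutline switch the mesh's Render Custom Depth flag, each first checking the Is Outline Active macro so that only actual state changes are applied.
; Interact only prints an on-screen debug message with the actor's display name.
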(event `Show Outline`
  ;[0.05 0.05 0.05 0.5] Show/Hide Outline
  (`self.Is Outline Active`
    (:`false`
      (`PrimitiveComponent.SetRenderCustomDepth` (`self.Mesh`) true))))

(event `Hide Outline`
  ;[0.05 0.05 0.05 0.5] Show/Hide Outline
  (`self.Is Outline Active`
    (:`true`
      (`PrimitiveComponent.SetRenderCustomDepth` (`self.Mesh`) false))))

(event `Interact`
  (`KismetSystemLibrary.PrintString` (`KismetStringLibrary.Concat_StrStr` "Interacting with: [" (`KismetSystemLibrary.GetDisplayName` self) "]") true true (struct :`R` 1.0 :`G` 0.5 :`A` 1.0) 15.0))

(fn `UserConstructionScript`)