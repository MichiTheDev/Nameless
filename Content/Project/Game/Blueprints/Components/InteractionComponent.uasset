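; InteractionComponent is an actor component that lets its owner highlight and use the BP_Interactable it is looking at.
; On BeginPlay it caches the owner's camera, printing a warning if none exists.
; Each tick it line-traces forward from the camera up to InteractionRange, storing the hit interactable and updating outlines as the target changes.
; The Interact event forwards to that stored target.
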(event `self.ReceiveBeginPlay`
  (bind _returnvalue (`self.GetOwner`))
  (bind _returnvalue_2 (`Actor.GetComponentByClass` _returnvalue "/Script/Engine.CameraComponent"))
  ;[0.05 0.05 0.05 0.5] Begin Play
  (`/Engine/EditorBlueprintResources/StandardMacros.IsValid` _returnvalue_2
    (:`Is Valid`
      (set `self.Camera` _returnvalue_2))
    (:`Is Not Valid`
      (`KismetSystemLibrary.PrintString` (`KismetStringLibrary.Concat_StrStr` (`KismetSystemLibrary.GetDisplayName` _returnvalue) " has no valid Camera. [PlayerPickupComponent] will disable itself.") true true (struct :`R` 1.0 :`A` 1.0) 15.0))))

(event `self.ReceiveTick`
  (params (DeltaSeconds :type "Float (single-precision)"))
  (bind _camera (`self.Camera`))
  (bind _returnvalue (`SceneComponent.K2_GetComponentLocation` _camera))
  ;[0.05 0.05 0.05 0.5] Event Tick
  (bind _outhit (`KismetSystemLibrary.LineTraceSingleForObjects` _returnvalue (+ _returnvalue (* (`SceneComponent.GetForwardVector` _camera) (`self.Interaction Range`))) (`|MakeArray` "ObjectTypeQuery2" "ObjectTypeQuery4" "ObjectTypeQuery1" :!type "EObjectTypeQuery Enum")))
  (bind _output_get (set `self.Latest Hit Result` _outhit))
  (bind _asbp_interactable (cast `/Game/Project/Game/Blueprints/Actors/Interactables/BP_Interactable` (`.HitActor` (`GameplayStatics.BreakHitResult` _output_get)))
    (:`then`
      (bind _interactable (`self.Interactable`)
        (:`then`
          (`/Game/Project/Game/Blueprints/Actors/Interactables/BP_Interactable.Hide Outline` _interactable))
        (:`else`
          _))
      (bind _output_get_2 (set `self.Interactable` _asbp_interactable))
      (`/Game/Project/Game/Blueprints/Actors/Interactables/BP_Interactable.Show Outline` _output_get_2))
    (:`CastFailed`
      (bind _interactable_2 (`self.Interactable`)
        (:`then`
          (`/Game/Project/Game/Blueprints/Actors/Interactables/BP_Interactable.Hide Outline` _interactable_2)
          (set `self.Interactable` null))
        (:`else`)))))

(event `Interact`
  ;[0.05 0.05 0.05 0.5] Interact
  (bind _interactable (`self.Interactable`)
    (:`then`
      (`/Game/Project/Game/Blueprints/Actors/Interactables/BP_Interactable.Interact` _interactable))
    (:`else`)))