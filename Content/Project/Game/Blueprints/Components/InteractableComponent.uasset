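; Actor component that makes its owner interactable, with a toggleable highlight outline.
; On BeginPlay it caches the owner's static mesh component, or prints a warning and deactivates itself if none exists.
; Show and hide events toggle the mesh's Render Custom Depth, guarded by an IsOutlineActive check.
; Interact broadcasts the OnInteract dispatcher with the player and prints a debug message.
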(event `self.ReceiveBeginPlay`
  (bind _returnvalue (`self.GetOwner`))
  (bind _returnvalue_2 (`Actor.GetComponentByClass` _returnvalue "/Script/Engine.StaticMeshComponent"))
  ;[0.05 0.05 0.05 0.5] Begin Play
  (`/Engine/EditorBlueprintResources/StandardMacros.IsValid` _returnvalue_2
    (:`Is Valid`
      (set `self.Mesh` _returnvalue_2))
    (:`Is Not Valid`
      (`KismetSystemLibrary.PrintString` (`KismetStringLibrary.Concat_StrStr` (`KismetSystemLibrary.GetDisplayName` _returnvalue) " has no valid Mesh. [InteractableComponent] will disable itself.") true true (struct :`R` 1.0 :`A` 1.0) 15.0)
      (`self.SetActive` false))))

(event `Show Outline`
  ;[0.05 0.05 0.05 0.5] Show/Hide Outline
  (`self.Is Outline Active`
    (:`false`
      (`PrimitiveComponent.SetRenderCustomDepth` (`self.Mesh`) true))))

(event `Hide Outline`
  ;[0.05 0.05 0.05 0.5] Show/Hide Outline
  (`self.Is Outline Active`
    (:`true`
      (`PrimitiveComponent.SetRenderCustomDepth` (`self.Mesh`) false))))

(event `Interact`
  (params (Player :type "PlayerController Object Reference"))
  ;[0.05 0.05 0.05 0.5] Interact
  (`self.OnInteract` Player)
  (`KismetSystemLibrary.PrintString` (`KismetStringLibrary.Concat_StrStr` "Interacting with: [" (`KismetSystemLibrary.GetDisplayName` self) "]") true true (struct :`R` 1.0 :`G` 0.5 :`A` 1.0) 15.0))