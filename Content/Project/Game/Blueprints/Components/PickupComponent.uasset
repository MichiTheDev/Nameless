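; Actor component that lets its owning actor be picked up and dropped by toggling physics and collision.
; On BeginPlay it caches the owner's primitive component, or prints a warning and deactivates itself if none exists.
; Pickup turns off physics simulation and actor collision, while Drop restores both and zeroes linear and angular velocity.
; Each action then fires its OnPickup or OnDrop notification.
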(event `self.ReceiveBeginPlay`
  (bind _returnvalue (`self.GetOwner`))
  (bind _returnvalue_2 (`Actor.GetComponentByClass` _returnvalue "/Script/Engine.PrimitiveComponent"))
  ;[0.05 0.05 0.05 0.5] Begin Play
  (`/Engine/EditorBlueprintResources/StandardMacros.IsValid` _returnvalue_2
    (:`Is Valid`
      (set `self.Primitive Component` _returnvalue_2))
    (:`Is Not Valid`
      (`KismetSystemLibrary.PrintString` (`KismetStringLibrary.Concat_StrStr` (`KismetSystemLibrary.GetDisplayName` _returnvalue) " has no primitive component. [PickupComponent] will disable itself.") true true (struct :`R` 1.0 :`A` 1.0) 15.0)
      (`self.SetActive` false))))

(fn `Drop`
  (`PrimitiveComponent.SetSimulatePhysics` (`self.Primitive Component`) true)
  (`Actor.SetActorEnableCollision` (`self.GetOwner`) true)
  (`PrimitiveComponent.SetPhysicsLinearVelocity` (`self.Primitive Component`) (0.0 0.0 0.0) false "None")
  (`PrimitiveComponent.SetPhysicsAngularVelocityInDegrees` (`self.Primitive Component`) (0.0 0.0 0.0) false "None")
  (`self.OnDrop`))

(fn `Pickup`
  (`PrimitiveComponent.SetSimulatePhysics` (`self.Primitive Component`) false)
  (`Actor.SetActorEnableCollision` (`self.GetOwner`) false)
  (`self.OnPickup`))